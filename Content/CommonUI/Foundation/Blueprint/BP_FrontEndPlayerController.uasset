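; Player controller for the front end that puts the UI container on screen and opens the main menu.
; On BeginPlay it adds UIContainer to the viewport and pushes UI_MainMenu onto it through PushMenuMessage.
; It exposes the container through GetUIContainer and toggles force feedback through a Vibration event.
; GetCamera is an empty stub that returns no value.
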(event `self.ReceiveBeginPlay`
  (bind _uicontainer (`self.UIContainer`))
  ;[1 0 0.7734] On Begin Play, Create the Container Widget and push the main menu
  (`parent.ReceiveBeginPlay`)
  (`UserWidget.AddToViewport` _uicontainer 0)
  (message `/Game/CommonUI/Foundation/Widgets/BPI_Container.PushMenu` _uicontainer "/Game/CommonUI/MainWidgets/UI_MainMenu.UI_MainMenu_C"))

(event `/Game/CommonUI/Settings/Widgets/BPI_PlayerController.Vibration`
  (params (Boolean :type Boolean))
  (set `self.bForceFeedbackEnabled` Boolean))

(fn `GetCamera`
  (returns (Camera :type "CameraComponent Object Reference"))
  (return null))

(fn `GetUIContainer`
  (returns (UIContainer :type "CommonActivatableWidget Object Reference"))
  (return (`self.UIContainer`)))

(fn `UserConstructionScript`
  (`parent.UserConstructionScript`))